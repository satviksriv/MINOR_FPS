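; Explosive barrel actor for an FPS that loses health from any damage and explodes when it runs out.
; Each hit shows a hit marker on the instigating player controller and lowers the HealthComponent's HP.
; At zero, a multicast event swaps in a physics-launched destroyed mesh with particles and sound.
; After short delays, it deals radial damage credited to the instigator, then destroys itself.
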(event `PlayEffects`
  (bind _barreldestroyedmesh (`self.BarrelDestroyedMesh`))
  (bind _returnvalue (`self.K2_GetActorLocation` self))
  ;[1 1 1] Multicast
  (`SceneComponent.SetVisibility` (`self.BarrelMesh`) false false)
  (`SceneComponent.SetVisibility` (`self.BarrelDestroyedMesh`) true false)
  (`GameplayStatics.SpawnEmitterAtLocation` "/Game/FPS/Effects/WeaponEffects/Explosion/P_Explosion.P_Explosion" _returnvalue (struct) (5.0 5.0 5.0))
  (`PrimitiveComponent.SetSimulatePhysics` _barreldestroyedmesh true)
  (`PrimitiveComponent.AddImpulseAtLocation` _barreldestroyedmesh (0.0 0.0 70000.0) _returnvalue "None")
  (`GameplayStatics.PlaySoundAtLocation` "/Game/FPS/MusicSound/Sounds/Explosions/Explosion_with_Metal_Debris.Explosion_with_Metal_Debris" _returnvalue (struct) 0.5 1.0 0.0 "/Game/FPS/MusicSound/Sounds/WeaponAttenuation.WeaponAttenuation" null null)
  (`ActorComponent.K2_DestroyComponent` (`self.HealthComponent`)))

(event `self.ReceiveBeginPlay`
  ;[1 1 1] Begin Play
  (`SceneComponent.SetVisibility` (`self.BarrelDestroyedMesh`) false false))

(event `self.ReceiveAnyDamage`
  (params (Damage :type "Float (single-precision)") (DamageType :type "DamageType Object Reference") (InstigatedBy :type "Controller Object Reference") (DamageCauser :type "Actor Object Reference"))
  (bind (_returnvalue_x _returnvalue_y _returnvalue_z) (`KismetMathLibrary.BreakVector` (`self.K2_GetActorLocation`)))
  ;[1 1 1] Any Damage
  (if (not (`self.bDestroyed`))
    (bind _explode (`self.TakeDamage` Damage InstigatedBy))
    (if _explode
      (set `self.bDestroyed` true)
      (`self.PlayEffects`)
      (`KismetSystemLibrary.Delay` 0.15)
      (`GameplayStatics.ApplyRadialDamage` 500.0 (`KismetMathLibrary.MakeVector` _returnvalue_x _returnvalue_y (+ _returnvalue_z 55.0)) 600.0 "/Game/FPS/Blueprints/Weapons/DamageTypes/DT_Explosion.DT_Explosion_C" (`|MakeArray` self :!type "Actor Object Reference") self InstigatedBy)
      (`KismetSystemLibrary.Delay` 8.0)
      (`self.K2_DestroyActor`))))

(fn `TakeDamage`
  (params (Dmg :type "Float (double-precision)") (NewParam :type "Controller Object Reference"))
  (returns (Explode :type Boolean))
  (bind _healthcomponent (`self.HealthComponent`))
  (bind _asbase_character_pc (cast `/Game/FPS/Blueprints/PlayerController/BaseCharacterPC` NewParam)
    (:`then`
      (`/Game/FPS/Blueprints/PlayerController/BaseCharacterPC.ShowHitMarker` _asbase_character_pc))
    (:`CastFailed`
      _))
  (bind _output_get (set `/Game/FPS/Blueprints/HealthComponent/HealthComponent.HP` (- (`/Game/FPS/Blueprints/HealthComponent/HealthComponent.HP` _healthcomponent) Dmg) _healthcomponent))
  (return (<= _output_get 0.0)))

(fn `UserConstructionScript`)